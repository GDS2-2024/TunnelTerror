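; Game state for Tunnel Terror that manages the match timer and the lobby-to-level transition in multiplayer.
; On the server, Tick counts GameTime down to zero while out of the lobby and in TestLevel1.
; ResetTimers restores the game and chaos timers on authority and flags the lobby state.
; CheckAllReady scans the lobby player states and server-travels to TestLevel1 once every player is ready.
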(event `self.ReceiveBeginPlay`)

(event `self.ReceiveTick`
  (params (DeltaSeconds :type "Float (single-precision)"))
  (if (`self.bInLobby`)
    _
    (elif (`self.bGameTime`)
      (`/Engine/EditorBlueprintResources/ActorMacros.Switch Has Authority`
        (:`Authority`
          (bind _returnvalue (`GameplayStatics.GetCurrentLevelName` true))
          (if (`KismetStringLibrary.EqualEqual_StrStr` _returnvalue "TestLevel1")
            (if (> (`self.gameTime`) 0.0)
              (set `self.gameTime` (- (`self.gameTime`) (`GameplayStatics.GetWorldDeltaSeconds`)))
              (else
                (set `self.gameTime` 0.0)))))))))

(event `self.ResetTimers`
  (`KismetSystemLibrary.PrintString` "Timers reset")
  (`/Engine/EditorBlueprintResources/ActorMacros.Switch Has Authority`
    (:`Authority`
      (set `self.gameTime` 600.0)
      (set `self.chaosTime` 30.0)
      (set `self.bInLobby` true))))

(fn `Check All Ready`
  (bind _playerarray (`self.PlayerArray`))
  (bind _returnvalue (`KismetArrayLibrary.Array_Length` _playerarray))
  (`KismetSystemLibrary.PrintString` (`KismetStringLibrary.Conv_IntToString` _returnvalue))
  (if (> _returnvalue 0)
    (for _array_element _playerarray
      (bind _aslobby_player_state (cast `/Game/Blueprints/LobbyPlayerState` _array_element))
      (if (not (`/Game/Blueprints/LobbyPlayerState.StateIsReady` _aslobby_player_state))
        (return)))
    (`KismetSystemLibrary.PrintString` "load lvl")
    (`AdvancedSessionsLibrary.ServerTravel` "TestLevel1")))

(fn `UserConstructionScript`)