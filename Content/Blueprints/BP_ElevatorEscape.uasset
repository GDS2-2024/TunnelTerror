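; Escape elevator actor with a sliding door and a screen that shows the current sample count.
; PlayDoorOpenAnimationImplementation runs a timeline that lerps the door downward in relative space.
; The SampleScreen widget component's ElevatorScreenWidget gets its text set from CurrentSamples, both every Tick and on UpdateSamplesIndicator.
; The Blueprint only handles these visuals and contains no sample counting or door trigger logic.
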(event `self.ReceiveTick`
  (params (DeltaSeconds :type "Float (single-precision)"))
  (bind _aselevator_screen_widget (cast `/Game/Blueprints/ElevatorScreenWidget` (`WidgetComponent.GetUserWidgetObject` (`self.SampleScreen`)) :!label _label))
  (`TextBlock.SetText` (`/Game/Blueprints/ElevatorScreenWidget.CurrentSamplesText` _aselevator_screen_widget) (`KismetTextLibrary.Conv_IntToText` (`self.currentSamples`))))

(event `self.PlayDoorOpenAnimationImplementation`
  (bind (_direction _open_door_anim) (`Timeline|Open Door`)
    (:`Update`
      (`SceneComponent.K2_SetRelativeLocation` (`self.Elevator Door`) (`KismetMathLibrary.VLerp` (0.0 0.0 0.0) (0.0 0.0 -200.0) _open_door_anim) false false))))

(event `UpdateSamplesIndicator`
  (goto _label))

(fn `UserConstructionScript`)