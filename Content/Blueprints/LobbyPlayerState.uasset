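; LobbyPlayerState tracks whether a player in the Tunnel Terror lobby is ready.
; Its SetStateReady event sets the StateIsReady flag from the incoming value and prints it for debugging.
; When the player becomes ready, it casts the game state to BP_TunnelTerrorGameState and calls CheckAllReady, while un-readying only clears the flag.
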(event `SetStateReady`
  (params (Ready :type Boolean))
  (`KismetSystemLibrary.PrintString` "setting ready")
  (if Ready
    (bind _output_get (set `self.StateIsReady` true))
    (`KismetSystemLibrary.PrintString` (`KismetStringLibrary.Conv_BoolToString` _output_get))
    (bind _asbp_tunnel_terror_game_state (cast `/Game/Blueprints/BP_TunnelTerrorGameState` (`GameplayStatics.GetGameState`)))
    (`/Game/Blueprints/BP_TunnelTerrorGameState.Check All Ready` _asbp_tunnel_terror_game_state)
    (else
      (bind _output_get_2 (set `self.StateIsReady` false))
      (`KismetSystemLibrary.PrintString` (`KismetStringLibrary.Conv_BoolToString` _output_get_2)))))

(fn `UserConstructionScript`)