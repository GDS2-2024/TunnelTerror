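; BP_SporePlant is a plant trap actor that relays death and snap states to its skeletal mesh animation.
; On BeginPlay it turns off its CanTimeOut flag.
; Its DeathAnim, Snap and StopSnap events cast the mesh's anim instance to AnimBP_PlantTrap and set the IsDying or IsSnapping flags.
; The graph holds no trigger or spore logic, so these events are not called within it.
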(event `self.ReceiveBeginPlay`
  (set `self.bCanTimeOut` false))

(event `self.DeathAnim`
  (bind _asanim_bp_plant_trap (cast `/Game/Blueprints/AnimationBP/AnimBP_PlantTrap` (`SkeletalMeshComponent.GetAnimInstance` (`self.SkeletalMesh`))))
  (set `/Game/Blueprints/AnimationBP/AnimBP_PlantTrap.isDying` true _asanim_bp_plant_trap))

(event `self.Snap`
  (bind _asanim_bp_plant_trap (cast `/Game/Blueprints/AnimationBP/AnimBP_PlantTrap` (`SkeletalMeshComponent.GetAnimInstance` (`self.SkeletalMesh`))))
  (set `/Game/Blueprints/AnimationBP/AnimBP_PlantTrap.isSnapping` true _asanim_bp_plant_trap))

(event `self.StopSnap`
  (bind _asanim_bp_plant_trap (cast `/Game/Blueprints/AnimationBP/AnimBP_PlantTrap` (`SkeletalMeshComponent.GetAnimInstance` (`self.SkeletalMesh`))))
  (set `/Game/Blueprints/AnimationBP/AnimBP_PlantTrap.isSnapping` false _asanim_bp_plant_trap))

(fn `UserConstructionScript`)